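; Level manager that tracks player progress through checkpoints across levels, each level being an entry in a nested array of locations.
; On BeginPlay it finds one current-platform and one next-platform actor, then reuses them by teleporting both as the checkpoint index changes.
; Reached and unreached events step that index forward or back, rolling between levels and printing messages at either end.
; A separate event teleports a given player just above the current checkpoint.
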(event Custom|levelCompleted
  ;[0.15 0.15 0.15 0.5] increment currentLevel and reset CCI
  (if (>= (+ (Variables|Default|GetcurrentLevel) 1) (Utilities|Array|Length (Variables|Default|GetallCheckpoints)))
    (Development|PrintString "You Win!")
    (else
      (Math|Integer|IncrementInt (Variables|Default|GetcurrentLevel)
        (:%20%20
          (Variables|Default|SetcurrentCheckpointIndex 0)
          (CallFunction|UpdateCheckpoints))))))

(event Custom|levelUncompleted
  ;[0.15 0.15 0.15 0.5] increment currentLevel and reset CCI
  (if (<= (Variables|Default|GetcurrentLevel) 0)
    (Development|PrintString "At Start")
    (else
      (bind _result (Math|Integer|DecrementInt (Variables|Default|GetcurrentLevel))
        (:%20%20
          (Variables|Default|SetcurrentCheckpointIndex (- (Utilities|Array|Length (.levelcheckpoints (Utilities|Array|Get(acopy) (Variables|Default|GetallCheckpoints) _result))) 1))
          (CallFunction|UpdateCheckpoints))))))

(event Custom|teleportPlayerToCheckpoint
  (params (playerToTeleport :type BP%20Third%20Person%20Character%20Object%20Reference))
  ;[0.15 0.15 0.15 0.5] teleports player to current checkpoint
  (Transformation|SetActorLocation playerToTeleport (+ (Variables|Default|GetcurrentCheckpointLocation) "0.000000,0.000000,100.000000") false true))

(event Custom|updateCheckpoints
  (bind _allcheckpoints (Variables|Default|GetallCheckpoints))
  (bind _currentlevel (Variables|Default|GetcurrentLevel))
  (bind _currentcheckpointindex (Variables|Default|GetcurrentCheckpointIndex))
  (bind _output (Utilities|Array|Get(acopy) _allcheckpoints _currentlevel))
  ;[0.15 0.15 0.15 0.5] update current and next checkpoint locations and platforms based on currentLevel and CCI
  (Utilities|FlowControl|Sequence
    (:then_0
      (bind _output_get (Variables|Default|SetnextCheckpointLocation (Utilities|Array|Get(acopy) (.levelcheckpoints _output) (+ _currentcheckpointindex 1))))
      (Transformation|SetActorLocation (Variables|Default|GetnextPlatRef) _output_get false true))
    (:then_1
      (bind _output_get_2 (Variables|Default|SetcurrentCheckpointLocation (Utilities|Array|Get(acopy) (.levelcheckpoints _output) _currentcheckpointindex)))
      (Transformation|SetActorLocation (Variables|Default|GetcurrentPlatRef) _output_get_2 false true))))

(event Custom|reverseCheckpoints
  (bind _allcheckpoints (Variables|Default|GetallCheckpoints))
  (bind _currentlevel (Variables|Default|GetcurrentLevel))
  (bind _currentcheckpointindex (Variables|Default|GetcurrentCheckpointIndex))
  (bind _output (Utilities|Array|Get(acopy) _allcheckpoints _currentlevel))
  ;[0.15 0.15 0.15 0.5] same as update but reverse
  (Utilities|FlowControl|Sequence
    (:then_0
      (bind _output_get (Variables|Default|SetnextCheckpointLocation (Utilities|Array|Get(acopy) (.levelcheckpoints _output) _currentcheckpointindex)))
      (Transformation|SetActorLocation (Variables|Default|GetnextPlatRef) _output_get false true))
    (:then_1
      (bind _output_get_2 (Variables|Default|SetcurrentCheckpointLocation (Utilities|Array|Get(acopy) (.levelcheckpoints _output) (- _currentcheckpointindex 1))))
      (Transformation|SetActorLocation (Variables|Default|GetcurrentPlatRef) _output_get_2 false true))))

(event Custom|checkpointReached
  ;[0.15 0.15 0.15 0.5] check if next checkpoint is last; if so, exe levelCompleted; otherwise, increment CCI and exe updateCheckpoints
  (if (== (+ (Variables|Default|GetcurrentCheckpointIndex) 2) (Utilities|Array|Length (.levelcheckpoints (Utilities|Array|Get(acopy) (Variables|Default|GetallCheckpoints) (Variables|Default|GetcurrentLevel)))))
    (CallFunction|LevelCompleted)
    (else
      (Math|Integer|IncrementInt (Variables|Default|GetcurrentCheckpointIndex)
        (:%20%20
          (CallFunction|UpdateCheckpoints))))))

(event Custom|checkpointUnreached
  ;[0.15 0.15 0.15 0.5] check if next checkpoint is last; if so, exe levelCompleted; otherwise, increment CCI and exe updateCheckpoints
  (if (<= (Variables|Default|GetcurrentCheckpointIndex) 0)
    (CallFunction|LevelUncompleted)
    (else
      (Math|Integer|DecrementInt (Variables|Default|GetcurrentCheckpointIndex)
        (:%20%20
          (CallFunction|ReverseCheckpoints))))))

(event EventBeginPlay
  ;[0.15 0.15 0.15 0.5] setup to get references to current and next platforms
  (bind _returnvalue (Actor|GetActorOfClass "/Game/bluePrints/BP_currentPlatform.BP_currentPlatform_C"))
  (Variables|Default|SetcurrentPlatRef _returnvalue)
  (bind _returnvalue_2 (Actor|GetActorOfClass "/Game/bluePrints/BP_nextPlatform.BP_nextPlatform_C"))
  (Variables|Default|SetnextPlatRef _returnvalue_2)
  (CallFunction|UpdateCheckpoints))

(fn ConstructionScript)