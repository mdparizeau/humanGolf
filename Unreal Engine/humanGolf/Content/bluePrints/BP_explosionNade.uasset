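; Explosive grenade actor that knocks characters away from the point where it hits.
; On Hit, it sphere-overlaps pawns of the BP_ThirdPersonCharacter class within BlastRadius of the hit location.
; Each one is launched directly away from that point at a fixed speed regardless of distance, added to its current velocity.
; It then prints a debug message and destroys itself, applying no damage.
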(event Collision|EventHit
  (params (MyComp :type Primitive%20Component%20Object%20Reference) (Other :type Actor%20Object%20Reference) (OtherComp :type Primitive%20Component%20Object%20Reference) (bSelfMoved :type Boolean) (HitLocation :type Vector :default "0, 0, 0") (HitNormal :type Vector :default "0, 0, 0") (NormalImpulse :type Vector :default "0, 0, 0") (Hit :type Hit%20Result%20Structure%20%28by%20ref%29))
  (bind _outactors (Collision|SphereOverlapActors HitLocation (Variables|Default|GetblastRadius) (Utilities|Array|MakeArray "ObjectTypeQuery3") "/Game/ThirdPerson/Blueprints/BP_ThirdPersonCharacter.BP_ThirdPersonCharacter_C"))
  (for _array_element _outactors
    (bind _asbp_third_person_character (Utilities|Casting|CastToBP_ThirdPersonCharacter _array_element))
    (Character|LaunchCharacter _asbp_third_person_character (* (Math|Vector|Normalize (- HitLocation (Transformation|GetActorLocation _asbp_third_person_character))) "-800.000000,-800.000000,-800.000000") false false))
  (Development|PrintString "EXLODE!!!")
  (Actor|DestroyActor))

(fn ConstructionScript)