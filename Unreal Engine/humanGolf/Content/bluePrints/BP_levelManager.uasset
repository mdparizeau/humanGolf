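; BP_levelManager tracks level and checkpoint progression through per-level checkpoint location lists.
; Reaching a checkpoint advances the index, or completes the level when the next checkpoint is the last one.
; Completing a level increments the current level and resets the index.
; Both paths then refresh the current and next checkpoint locations from the AllCheckpoints array, with no check for running past the final level.
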(event Custom|updateCheckpoints
  (bind _allcheckpoints (Variables|Default|GetallCheckpoints))
  (bind _currentlevel (Variables|Default|GetcurrentLevel))
  (bind _currentcheckpointindex (Variables|Default|GetcurrentCheckpointIndex))
  (bind _output (Utilities|Array|Get(acopy) _allcheckpoints _currentlevel))
  ;[0.15 0.15 0.15 0.5] update current and next checkpoint locations based on currentLevel and CCI
  (Utilities|FlowControl|Sequence
    (:then_0
      (Variables|Default|SetnextCheckpointLocation (Utilities|Array|Get(acopy) (.levelcheckpoints _output) (+ _currentcheckpointindex 1))))
    (:then_1
      (Variables|Default|SetcurrentCheckpointLocation (Utilities|Array|Get(acopy) (.levelcheckpoints _output) _currentcheckpointindex)))))

(event Custom|levelCompleted
  ;[0.15 0.15 0.15 0.5] increment currentLevel and reset CCI
  (Math|Integer|IncrementInt (Variables|Default|GetcurrentLevel)
    (:%20%20
      (Variables|Default|SetcurrentCheckpointIndex 0)
      (CallFunction|UpdateCheckpoints))))

(event Custom|checkpointReached
  ;[0.15 0.15 0.15 0.5] check if next checkpoint is last; if so, exe levelCompleted; otherwise, increment CCI and exe updateCheckpoints
  (if (== (+ (Variables|Default|GetcurrentCheckpointIndex) 2) (Utilities|Array|Length (.levelcheckpoints (Utilities|Array|Get(acopy) (Variables|Default|GetallCheckpoints) (Variables|Default|GetcurrentLevel)))))
    (CallFunction|LevelCompleted)
    (else
      (Math|Integer|IncrementInt (Variables|Default|GetcurrentCheckpointIndex)
        (:%20%20
          (CallFunction|UpdateCheckpoints))))))

(fn ConstructionScript)